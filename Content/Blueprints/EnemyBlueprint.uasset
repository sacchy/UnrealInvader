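; EnemyBlueprint is an enemy actor that patrols back and forth along the world Y axis.
; Each Tick it offsets its location at a constant speed, scaled by DeltaSeconds and the DirectionY sign, without sweeping for collision.
; DirectionY flips when the actor passes fixed bounds on either side of the world origin, so the patrol range is absolute rather than relative to its spawn point.
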(event EventBeginPlay)

(event EventActorBeginOverlap
  (params (OtherActor :type Actor%20Object%20Reference)))

(event EventTick
  (params (DeltaSeconds :type Float%20%28single-precision%29))
  (bind _returnvalue (Transformation|GetActorLocation))
  (bind _y (Math|Vector|BreakVector _returnvalue))
  ;[1 1 1] 敵の移動処理
  (Transformation|SetActorLocation (+ (* (* "0,50.000000, 0" DeltaSeconds) (* "0,1.000000, 0" (Variables|Default|GetDirectionY))) (Transformation|GetActorLocation)) false)
  ;[1 1 1] 移動方向変更処理
  (if (< 1e+02 _y)
    (Variables|Default|SetDirectionY -1.0)
    (elif (> -1e+02 _y)
      (Variables|Default|SetDirectionY 1.0))))

(fn ConstructionScript)